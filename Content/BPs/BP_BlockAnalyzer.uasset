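; Slot detector for a block-chaining puzzle that records the tagged block attached to it and judges the level's answer.
; Button, energy and light sensor events look up the analyzer with the next index among all analyzers.
; If this analyzer holds an energy block, it drives that next block: toggling light or fan by click parity, ringing sound, or lighting energy.
; Activated outputs are compared with the level's winning block, reporting to BP_WinLevelManager until won.
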(event `self.ReceiveBeginPlay`
  (bind _outactors (`GameplayStatics.GetAllActorsOfClass` "BP_BlockAnalyzer_C"))
  (set `self.OtherAnalyzersArray` _outactors)
  (set `self.clickCounter` 0.0)
  (set `self.WinPerLvlCounter` 0))

(fn `Button Pressed Event`
  (bind _generalactorindex (`self.CheckAnalyzerPosition`)
    (:`NotTheLast`
      (bind _nextblockanalyzer (`self.GetNextBlockAnalyzer` _generalactorindex))
      (`self.ReceiveButtonClickInput` _nextblockanalyzer))))

(fn `CallWinManager`
  (bind _returnvalue (`GameplayStatics.GetActorOfClass` "/Game/BPs/BP_WinLevelManager.BP_WinLevelManager_C"))
  (`/Engine/EditorBlueprintResources/StandardMacros.IsValid` _returnvalue
    (:`Is Valid`
      (`/Engine/EditorBlueprintResources/StandardMacros.IncrementInt` (`self.WinPerLvlCounter`)
        (:`  `
          (`/Game/BPs/BP_WinLevelManager.WinLevelMessage` _returnvalue))))
    (:`Is Not Valid`
      (`KismetSystemLibrary.PrintString` "--------------------------LVL MANAGER NOT IN THE LEVEL"))))

(fn `CallWrongAnswerManager`
  (bind _returnvalue (`GameplayStatics.GetActorOfClass` "/Game/BPs/BP_WinLevelManager.BP_WinLevelManager_C"))
  (`/Engine/EditorBlueprintResources/StandardMacros.IsValid` _returnvalue
    (:`Is Valid`
      (`/Game/BPs/BP_WinLevelManager.WrongAsnwerMessage` _returnvalue))
    (:`Is Not Valid`
      (`KismetSystemLibrary.PrintString` "--------------------------LVL MANAGER NOT IN THE LEVEL"))))

(fn `EnergyBlockConnectionEvent`
  (bind _generalactorindex (`self.CheckAnalyzerPosition`)
    (:`NotTheLast`
      (bind _nextblockanalyzer (`self.GetNextBlockAnalyzer` _generalactorindex))
      (`self.ReceiveButtonClickInput` _nextblockanalyzer))))

(fn `LightSensorEvent`
  (bind _generalactorindex (`self.CheckAnalyzerPosition`)
    (:`NotTheLast`
      (bind _nextblockanalyzer (`self.GetNextBlockAnalyzer` _generalactorindex))
      (`self.ReceiveButtonClickInput` _nextblockanalyzer))))

(fn `ReceiveButtonClickInput`
  (params (NextBlockAnalyzerInArray :type "/Game/BPs/BP_BlockAnalyzer Object Reference"))
  (bind _block_reference (`/Game/BPs/BP_BlockAnalyzer.Block Reference` NextBlockAnalyzerInArray))
  (`self.CheckIfCurrentBlockIsEnergy`
    (:`IsEnergy`
      (switch `int` (`/Game/BPs/BP_BlockAnalyzer.CurrentlyAttachedBlockType` NextBlockAnalyzerInArray) ; 0==btn\n1==light\n2==energy\n3==fan\n4==Sound\n5==light sensor
        (:`1`
          (bind _asbp_light_block (cast `/Game/BPs/BlocksBP/BP_LightBlock` _block_reference))
          (`self.CheckClickEvenOdd`
            (:`even`
              (`/Game/BPs/BlocksBP/BP_LightBlock.TurnLightOff` _asbp_light_block))
            (:`odd`
              (`/Game/BPs/BlocksBP/BP_LightBlock.TurnLightOn` _asbp_light_block)
              (`self.CheckIfWonLevel` (`self.LightType`)))))
        (:`2`
          (bind _asbp_energy_block (cast `/Game/BPs/BlocksBP/BP_EnergyBlock` _block_reference))
          (`/Game/BPs/BlocksBP/BP_EnergyBlock.TurnEnergyIconOn` _asbp_energy_block))
        (:`3`
          (bind _asbp_fan_block (cast `/Game/BPs/BlocksBP/BP_FanBlock` _block_reference))
          (`self.CheckClickEvenOdd`
            (:`even`
              (`/Game/BPs/BlocksBP/BP_FanBlock.StopFan` _asbp_fan_block))
            (:`odd`
              (`/Game/BPs/BlocksBP/BP_FanBlock.MoveFan` _asbp_fan_block)
              (`self.CheckIfWonLevel` (`self.FanType`)))))
        (:`4`
          (bind _asbp_sound_block (cast `/Game/BPs/BlocksBP/BP_SoundBlock` _block_reference))
          (`/Game/BPs/BlocksBP/BP_SoundBlock.PlayBellSound` _asbp_sound_block)
          (`self.CheckIfWonLevel` (`self.SoundType`)))))))

(fn `SaveTouchedBlock`
  (params (BlockRefeence :type "/Game/BPs/BlocksBP/BP_BlockBase Object Reference"))
  (bind _output_get (set `self.Block Reference` BlockRefeence))
  (`self.SetBlockType` _output_get (`self.GeneralActorIndex`)))

(fn `SetBlockType`
  (params (BlockObj :type "/Game/BPs/BlocksBP/BP_BlockBase Object Reference") (DetectionBoxIndex :type Integer))
  (switch `name` (`|GetArrayItem` (`Actor.Tags` BlockObj))
    (:`Button`
      (set `self.CurrentlyAttachedBlockType` 0))
    (:`Light`
      (set `self.CurrentlyAttachedBlockType` 1))
    (:`Energy`
      (set `self.CurrentlyAttachedBlockType` 2))
    (:`Fan`
      (set `self.CurrentlyAttachedBlockType` 3))
    (:`Sound`
      (set `self.CurrentlyAttachedBlockType` 4))
    (:`LightSensor`
      (set `self.CurrentlyAttachedBlockType` 5))))

(fn `UserConstructionScript`)