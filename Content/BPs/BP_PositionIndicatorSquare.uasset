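; BP_PositionIndicatorSquare is an actor, named as a position indicator, that has logic to adjust its height for a seated player state.
; GetgameInstanceRef caches BP_DataGameInstance, and SetLocationBasedOnCharPosition reads its Seated flag to raise the root component by a fixed Z offset.
; Both calls sit disconnected in the event graph and BeginPlay is empty, so the height adjustment never runs from this Blueprint.
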(event `self.ReceiveBeginPlay`)

(fn `GetgameInstanceRef`
  (bind _asgame_instance (cast `GameInstance` (`GameplayStatics.GetGameInstance`)))
  (bind _asbp_data_game_instance (cast `/Game/BPs/UI/BP_DataGameInstance` _asgame_instance))
  (set `self.As BP Data Game Instance` _asbp_data_game_instance))

(fn `Set Location Based On Char Position`
  (bind _defaultsceneroot (`self.DefaultSceneRoot`))
  (bind (_returnvalue_x _returnvalue_y _returnvalue_z) (`KismetMathLibrary.BreakVector` (`SceneComponent.K2_GetComponentLocation` _defaultsceneroot)))
  (if (`/Game/BPs/UI/BP_DataGameInstance.Seated` (`self.As BP Data Game Instance`))
    (`SceneComponent.K2_SetWorldLocation` _defaultsceneroot (`KismetMathLibrary.MakeVector` _returnvalue_x _returnvalue_y (+ _returnvalue_z 50.0)) false false)))

(fn `UserConstructionScript`)