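; BP_LevelImg is an actor that displays a level image and a help image for that level through two widget components.
; On BeginPlay it casts each component's widget and applies the assigned brush assets.
; ShowHideHelpImage sets the help widget's visibility.
; Logic to fetch BP_DataGameInstance and raise the actor's root when Seated exists, but its EventGraph calls are unconnected and never run.
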(event `self.ReceiveBeginPlay`
  (`self.SetLevelImage`)
  (`self.SetLevelHelpImage`))

(fn `GetgameInstanceRef`
  (bind _asgame_instance (cast `GameInstance` (`GameplayStatics.GetGameInstance`)))
  (bind _asbp_data_game_instance (cast `/Game/BPs/UI/BP_DataGameInstance` _asgame_instance))
  (set `self.As BP Data Game Instance` _asbp_data_game_instance))

(fn `SetLevelHelpImage`
  (bind _aswbp_lvl_help_img (cast `/Game/BPs/UI/WBP_LvlHelpImg` (`WidgetComponent.GetWidget` (`self.LvlHelpImgWidget`))))
  (`Image.SetBrushFromAsset` (`/Game/BPs/UI/WBP_LvlHelpImg.LvlHelpImg` _aswbp_lvl_help_img) (`self.CurrentLevelHelpImage`)))

(fn `SetLevelImage`
  (bind _aswbp_lvl_img (cast `/Game/BPs/UI/WBP_LvlImg` (`WidgetComponent.GetWidget` (`self.LvlImgWidget`))))
  (`Image.SetBrushFromAsset` (`/Game/BPs/UI/WBP_LvlImg.LvlImg` _aswbp_lvl_img) (`self.CurrentLevelImage`)))

(fn `SetPositionBasedOnChar`
  (bind _defaultsceneroot (`self.DefaultSceneRoot`))
  (bind (_returnvalue_x _returnvalue_y _returnvalue_z) (`KismetMathLibrary.BreakVector` (`SceneComponent.K2_GetComponentLocation` _defaultsceneroot)))
  (if (`/Game/BPs/UI/BP_DataGameInstance.Seated` (`self.As BP Data Game Instance`))
    (`SceneComponent.K2_SetWorldLocation` _defaultsceneroot (`KismetMathLibrary.MakeVector` _returnvalue_x _returnvalue_y (+ _returnvalue_z 50.0)) false false)))

(fn `ShowHideHelpImage`
  (params (input :type Boolean))
  (`SceneComponent.SetVisibility` (`self.LvlHelpImgWidget`) input false))

(fn `UserConstructionScript`)