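; BP_BlockBase is a physics-simulated, grippable VR block that snaps onto a BP_BlockAnalyzer.
; It stores the gripping controller, and on box overlap registers itself with the analyzer and has that controller drop and socket it to the analyzer's mesh.
; Ending the overlap resets the analyzer's attached block type to -1.
; A helper returns the parent analyzer; game-instance-driven height adjustment for seated play exists but never runs.
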(event `VRGripInterface.OnGrip`
  (params (GrippingController :type "GripMotionControllerComponent Object Reference") (GripInformation :type "BPActorGripInformation Structure (by ref)"))
  ;[1 1 1] Get  current gripping controller reference
  (set `self.CurrentGripController` GrippingController))

(event `self.ReceiveBeginPlay`
  (`PrimitiveComponent.SetSimulatePhysics` (`self.StaticMeshComponent`) true))

(event `self.Box.OnComponentBeginOverlap`
  (params (OverlappedComponent :type "PrimitiveComponent Object Reference") (OtherActor :type "Actor Object Reference") (OtherComp :type "PrimitiveComponent Object Reference") (OtherBodyIndex :type Integer) (bFromSweep :type Boolean) (SweepResult :type "HitResult Structure (by ref)"))
  ;[1 1 1] Analyzer touch control events
  (bind _asbp_block_analyzer (cast `/Game/BPs/BP_BlockAnalyzer` OtherActor))
  (`/Game/BPs/BP_BlockAnalyzer.SaveTouchedBlock` _asbp_block_analyzer self)
  (`GripMotionControllerComponent.DropAndSocketObject` (`self.CurrentGripController`) (make `Transform_NetQuantize` (0.0 0.0 10.0) (struct) (1.25 1.25 1.25)) self 0 (`/Game/BPs/BP_BlockAnalyzer.AnBlockMesh` _asbp_block_analyzer) "None" true))

(event `self.Box.OnComponentEndOverlap`
  (params (OverlappedComponent :type "PrimitiveComponent Object Reference") (OtherActor :type "Actor Object Reference") (OtherComp :type "PrimitiveComponent Object Reference") (OtherBodyIndex :type Integer))
  ;[1 1 1] Analyzer touch control events
  (bind _asbp_block_analyzer (cast `/Game/BPs/BP_BlockAnalyzer` OtherActor))
  (set `/Game/BPs/BP_BlockAnalyzer.CurrentlyAttachedBlockType` -1 _asbp_block_analyzer))

(fn `GetgameInstanceRef`
  (bind _asgame_instance (cast `GameInstance` (`GameplayStatics.GetGameInstance`)))
  (bind _asbp_data_game_instance (cast `/Game/BPs/UI/BP_DataGameInstance` _asgame_instance))
  (set `self.As BP Data Game Instance` _asbp_data_game_instance))

(fn `GetParentAnalyzer`
  (returns (`AsBP Block Analyzer` :type "/Game/BPs/BP_BlockAnalyzer Object Reference"))
  (bind _asbp_block_analyzer (cast `/Game/BPs/BP_BlockAnalyzer` (`self.GetAttachParentActor`)))
  (return _asbp_block_analyzer))

(fn `Set Location Based On Char Position`
  (bind _staticmeshcomponent (`self.StaticMeshComponent`))
  (bind (_returnvalue_x _returnvalue_y _returnvalue_z) (`KismetMathLibrary.BreakVector` (`SceneComponent.K2_GetComponentLocation` _staticmeshcomponent)))
  (if (`/Game/BPs/UI/BP_DataGameInstance.Seated` (`self.As BP Data Game Instance`))
    (`SceneComponent.K2_SetWorldLocation` _staticmeshcomponent (`KismetMathLibrary.MakeVector` _returnvalue_x _returnvalue_y (+ _returnvalue_z 50.0)) false false)))

(fn `UserConstructionScript`)