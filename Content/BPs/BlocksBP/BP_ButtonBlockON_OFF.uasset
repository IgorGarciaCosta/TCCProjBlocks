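; BP_ButtonBlockON_OFF is a button block that forwards VR button state changes to the block analyzer it is attached to.
; When its VRButton component changes state, it casts its attach parent actor to BP_BlockAnalyzer and calls ButtonPressedEvent.
; It passes no state along, and does nothing if the parent is not an analyzer.
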(event `self.ReceiveBeginPlay`
  (`parent.ReceiveBeginPlay`))

(event `self.VRButton.OnButtonStateChanged`
  (params (ButtonState :type Boolean) (InteractingActor :type "Actor Object Reference") (InteractingComponent :type "PrimitiveComponent Object Reference"))
  (bind _asbp_block_analyzer (cast `/Game/BPs/BP_BlockAnalyzer` (`self.GetAttachParentActor`)))
  (`/Game/BPs/BP_BlockAnalyzer.Button Pressed Event` _asbp_block_analyzer))

(fn `UserConstructionScript`
  (`parent.UserConstructionScript`))