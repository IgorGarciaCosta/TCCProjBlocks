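; BP_LightBlock is a block with a light bulb that reports a win to the level when lit.
; TurnLightOn toggles the LightBulb component's visibility, then calls CallWinManager.
; CallWinManager finds the BP_WinLevelManager actor by class and sends it WinLevelMessage, printing a debug string if none exists.
; The toggle flips the current state, so it assumes the bulb starts hidden.
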(event `self.ReceiveBeginPlay`
  (`parent.ReceiveBeginPlay`))

(fn `CallWinManager`
  (bind _returnvalue (`GameplayStatics.GetActorOfClass` "/Game/BPs/BP_WinLevelManager.BP_WinLevelManager_C"))
  (`/Engine/EditorBlueprintResources/StandardMacros.IsValid` _returnvalue
    (:`Is Valid`
      (`/Game/BPs/BP_WinLevelManager.WinLevelMessage` _returnvalue))
    (:`Is Not Valid`
      (`KismetSystemLibrary.PrintString` "--------------------------LVL MANAGER NOT IN THE LEVEL"))))

(fn `TurnLightOn`
  (`SceneComponent.ToggleVisibility` (`self.LightBulb`) false)
  (`self.CallWinManager`))

(fn `UserConstructionScript`
  (`parent.UserConstructionScript`))