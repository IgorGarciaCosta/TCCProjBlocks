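; Fan block actor whose static mesh spins when switched on and starts stationary at BeginPlay.
; MoveFan and StopFan events toggle a RotatingMovement component between a fixed spin rate and zero.
; The fan also stops when a BP_BlockAnalyzer leaves its Box trigger.
; CallWinManager can send a win message to the level's BP_WinLevelManager, but nothing in this graph calls it.
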(event `self.ReceiveBeginPlay`
  (`MovementComponent.SetUpdatedComponent` (`self.RotatingMovement`) (`self.StaticMesh`))
  (`self.TurnfanOff`))

(event `self.ReceiveTick`
  (params (DeltaSeconds :type "Float (single-precision)")))

(event `MoveFan`
  (`self.TurnFanOn`))

(event `StopFan`
  (`self.TurnfanOff`))

(event `self.Box.OnComponentEndOverlap`
  (params (OverlappedComponent :type "PrimitiveComponent Object Reference") (OtherActor :type "Actor Object Reference") (OtherComp :type "PrimitiveComponent Object Reference") (OtherBodyIndex :type Integer))
  (cast `/Game/BPs/BP_BlockAnalyzer` OtherActor)
  (`self.TurnfanOff`))

(fn `CallWinManager`
  (bind _returnvalue (`GameplayStatics.GetActorOfClass` "/Game/BPs/BP_WinLevelManager.BP_WinLevelManager_C"))
  (`/Engine/EditorBlueprintResources/StandardMacros.IsValid` _returnvalue
    (:`Is Valid`
      (`/Game/BPs/BP_WinLevelManager.WinLevelMessage` _returnvalue))
    (:`Is Not Valid`
      (`KismetSystemLibrary.PrintString` "--------------------------LVL MANAGER NOT IN THE LEVEL"))))

(fn `TurnfanOff`
  (set `RotatingMovementComponent.RotationRate` (struct) (`self.RotatingMovement`)))

(fn `TurnFanOn`
  (set `RotatingMovementComponent.RotationRate` (struct :`Pitch` 420.0) (`self.RotatingMovement`)))

(fn `UserConstructionScript`
  (`parent.UserConstructionScript`))