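; BP_MagnetSensorBlock is a sensor block that detects actors tagged "magnet" entering or leaving its sphere.
; While LevelMainInput is true, both begin and end overlaps fire the same OnMagnetNear event.
; That event casts the attach parent to BP_BlockAnalyzer and calls its ButtonPressedEvent, so the magnet's arrival and departure each register as a button press.
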(event `OnMagnetNear`
  (bind _asbp_block_analyzer (cast `/Game/BPs/BP_BlockAnalyzer` (`self.GetAttachParentActor`)))
  (`/Game/BPs/BP_BlockAnalyzer.Button Pressed Event` _asbp_block_analyzer))

(event `self.Sphere.OnComponentBeginOverlap`
  (params (OverlappedComponent :type "PrimitiveComponent Object Reference") (OtherActor :type "Actor Object Reference") (OtherComp :type "PrimitiveComponent Object Reference") (OtherBodyIndex :type Integer) (bFromSweep :type Boolean) (SweepResult :type "HitResult Structure (by ref)"))
  ;[1 1 1] Get magnet near
  (if (`self.LevelMainInput`)
    (if (`self.ActorHasTag` OtherActor "magnet")
      (`self.OnMagnetNear`))))

(event `self.Sphere.OnComponentEndOverlap`
  (params (OverlappedComponent :type "PrimitiveComponent Object Reference") (OtherActor :type "Actor Object Reference") (OtherComp :type "PrimitiveComponent Object Reference") (OtherBodyIndex :type Integer))
  ;[1 1 1] Get magnet near
  (if (`self.LevelMainInput`)
    (if (`self.ActorHasTag` OtherActor "magnet")
      (`self.OnMagnetNear`))))

(fn `UserConstructionScript`
  (`parent.UserConstructionScript`))