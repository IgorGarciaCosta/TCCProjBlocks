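; VR hand-tracking character that lets the player click world-space widgets by touching them with hand spheres.
; When either sphere begins overlapping a WidgetComponent, both widget interaction components simulate a left mouse click.
; Each touch then calls ManageScreenFade, which plays a fade level sequence if TouchedButton is set and clears the flag.
; Up and Down keys adjust the capsule half height in fixed steps.
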(event `self.SphereLeft.OnComponentBeginOverlap`
  (params (OverlappedComponent :type "PrimitiveComponent Object Reference") (OtherActor :type "Actor Object Reference") (OtherComp :type "PrimitiveComponent Object Reference") (OtherBodyIndex :type Integer) (bFromSweep :type Boolean) (SweepResult :type "HitResult Structure (by ref)"))
  (bind _widgetinteractionleft (`self.WidgetInteractionLeft`))
  ;[1 1 1] Manages screen touches
  (cast `WidgetComponent` OtherComp)
  (`WidgetInteractionComponent.PressPointerKey` _widgetinteractionleft "LeftMouseButton")
  (`WidgetInteractionComponent.PressPointerKey` (`self.WidgetInteractionRight`) "LeftMouseButton")
  (`WidgetInteractionComponent.ReleasePointerKey` _widgetinteractionleft "LeftMouseButton")
  (`WidgetInteractionComponent.ReleasePointerKey` (`self.WidgetInteractionRight`) "LeftMouseButton")
  (`self.ManageScreenFade`))

(event `self.SphereRight.OnComponentBeginOverlap`
  (params (OverlappedComponent :type "PrimitiveComponent Object Reference") (OtherActor :type "Actor Object Reference") (OtherComp :type "PrimitiveComponent Object Reference") (OtherBodyIndex :type Integer) (bFromSweep :type Boolean) (SweepResult :type "HitResult Structure (by ref)"))
  (bind _widgetinteractionleft (`self.WidgetInteractionLeft`))
  ;[1 1 1] Manages screen touches
  (cast `WidgetComponent` OtherComp)
  (`WidgetInteractionComponent.PressPointerKey` _widgetinteractionleft "LeftMouseButton")
  (`WidgetInteractionComponent.PressPointerKey` (`self.WidgetInteractionRight`) "LeftMouseButton")
  (`WidgetInteractionComponent.ReleasePointerKey` _widgetinteractionleft "LeftMouseButton")
  (`WidgetInteractionComponent.ReleasePointerKey` (`self.WidgetInteractionRight`) "LeftMouseButton")
  (`self.ManageScreenFade`))

(event `Key|Down`
  (params (Key :type "Key Structure"))
  (bind _capsulecomponent (`self.CapsuleComponent`))
  ;[1 1 1] Increase/Decrease capsule half height by clicking buttons
  (:`Pressed`
    (`CapsuleComponent.SetCapsuleHalfHeight` _capsulecomponent (- (`CapsuleComponent.CapsuleHalfHeight` _capsulecomponent) 5.0) true)))

(event `Key|Up`
  (params (Key :type "Key Structure"))
  (bind _capsulecomponent (`self.CapsuleComponent`))
  ;[1 1 1] Increase/Decrease capsule half height by clicking buttons
  (:`Pressed`
    (`CapsuleComponent.SetCapsuleHalfHeight` _capsulecomponent (+ (`CapsuleComponent.CapsuleHalfHeight` _capsulecomponent) 5.0) true)))

(event `ManageScreenFade`
  ;[1 1 1] Manage screen fade
  (if (`self.TouchedButton`)
    (bind _outactor (`LevelSequencePlayer.CreateLevelSequencePlayer` "/Game/BPs/FadeSequence.FadeSequence"))
    (`MovieSceneSequencePlayer.PlayTo` :`self` (`LevelSequenceActor.SequencePlayer` _outactor))
    (set `self.TouchedButton` false)))

(fn `UserConstructionScript`)