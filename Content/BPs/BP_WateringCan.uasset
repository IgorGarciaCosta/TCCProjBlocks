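; BP_WateringCan is a watering can actor that switches its water-falling particles on and off.
; Each tick, a 1000-unit line trace on a custom channel runs along the LineTraceRef component's forward vector.
; A hit activates the particles and sets PouringWater; a miss clears both.
; Functions to cache BP_DataGameInstance and raise the mesh for a seated player exist but are never called.
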(event `self.ReceiveBeginPlay`)

(event `self.ReceiveTick`
  (params (DeltaSeconds :type "Float (single-precision)"))
  (`self.ManageParticleSystemActivation`))

(fn `GetgameInstanceRef`
  (bind _asgame_instance (cast `GameInstance` (`GameplayStatics.GetGameInstance`)))
  (bind _asbp_data_game_instance (cast `/Game/BPs/UI/BP_DataGameInstance` _asgame_instance))
  (set `self.As BP Data Game Instance` _asbp_data_game_instance))

(fn `ManageParticleSystemActivation`
  (bind _waterfallingparticles (`self.WaterFallingParticles`))
  (bind _linetraceref (`self.LineTraceRef`))
  (bind _returnvalue (`SceneComponent.K2_GetComponentLocation` _linetraceref))
  (bind (_outhit _returnvalue_2) (`KismetSystemLibrary.LineTraceSingle` _returnvalue (+ _returnvalue (* (`SceneComponent.GetForwardVector` _linetraceref) 1000.0)) "TraceTypeQuery4"))
  (if _returnvalue_2
    (`ActorComponent.SetActive` _waterfallingparticles true false)
    (set `self.PouringWater` true)
    (else
      (`ActorComponent.SetActive` _waterfallingparticles false false)
      (set `self.PouringWater` false))))

(fn `SetPositionBasedOnChar`
  (bind _staticmeshcomponent (`self.StaticMeshComponent`))
  (bind (_returnvalue_x _returnvalue_y _returnvalue_z) (`KismetMathLibrary.BreakVector` (`SceneComponent.K2_GetComponentLocation` _staticmeshcomponent)))
  (if (`/Game/BPs/UI/BP_DataGameInstance.Seated` (`self.As BP Data Game Instance`))
    (`SceneComponent.K2_SetWorldLocation` _staticmeshcomponent (`KismetMathLibrary.MakeVector` _returnvalue_x _returnvalue_y (+ _returnvalue_z 50.0)) false false)))

(fn `UserConstructionScript`)